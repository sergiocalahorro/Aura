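; BP_FireBall is the Fire Blast fireball projectile, which flies out and returns to its instigator like a boomerang.
; StartMovement runs only with authority, driving an outgoing timeline that lerps the actor forward by TravelDistance from its start location.
; A returning timeline then lerps from that apex toward the instigator's live location, without sweeping.
; Once within ExplodeDistance of the instigator, it calls ProjectileHit and destroys itself.
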(event EventStartMovement
  (bind _returnvalue (Transformation|GetActorLocation))
  (Networking|SwitchHasAuthority
    (:Authority
      (Variables|Default|SetInitialLocation _returnvalue)
      (Variables|Default|SetApexLocation (+ _returnvalue (* (Transformation|GetActorForwardVector) (Variables|Default|GetTravelDistance))))
      (bind _alpha (Timeline|OutgoingTimeline Play)
        (:Update
          (Transformation|SetActorLocation (Math|Vector|Lerp(Vector) (Variables|Default|GetInitialLocation) (Variables|Default|GetApexLocation) _alpha) false false))
        (:Finished
          (bind _alpha_2 (Timeline|ReturningTimeline Play)
            (:Update
              (Transformation|SetActorLocation (Math|Vector|Lerp(Vector) (Variables|Default|GetApexLocation) (Transformation|GetActorLocation (Game|GetInstigator)) _alpha_2) false false)
              (if (CallFunction|IsWithinExplodeDistance)
                (Class|AuraProjectile|ProjectileHit)
                (Actor|DestroyActor)))))))))

(fn ConstructionScript)

(fn IsWithinExplodeDistance
  (return (<= (Transformation|GetDistanceTo (Game|GetInstigator)) (Variables|Default|GetExplodeDistance))))