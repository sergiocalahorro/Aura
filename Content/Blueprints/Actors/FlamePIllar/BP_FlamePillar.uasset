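; BP_FlamePillar is a flame pillar actor whose FlameLight flickers by scaling BaseIntensity with a timeline curve.
; After a random initial delay on BeginPlay, FlameIntensityTimeline ping-pongs endlessly, alternating forward and reverse when it finishes.
; CalculateRandomTimelineSpeed resets the play rate before each pass, but both random bounds use MinTimelinePlayRate, so the speed does not actually vary.
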(event EventBeginPlay
  (Utilities|FlowControl|Delay (Math|Random|RandomFloatinRange 0.0 (Variables|Default|GetMaxInitialDelay)))
  (CallFunction|CalculateRandomTimelineSpeed)
  (bind (_direction _flameintensity) (Timeline|FlameIntensityTimeline PlayFromStart)
    (:Update
      (Rendering|Components|Light|SetIntensity (Variables|Default|GetFlameLight) (* (Variables|Default|GetBaseIntensity) _flameintensity)))
    (:Finished
      (switch Utilities|FlowControl|Switch|SwitchonETimelineDirection _direction
        (:Forward
          (CallFunction|CalculateRandomTimelineSpeed)
          (Components|Timeline|ReversefromEnd (Variables|Default|GetFlameIntensityTimeline)))
        (:Backward
          (CallFunction|CalculateRandomTimelineSpeed)
          (Components|Timeline|PlayfromStart (Variables|Default|GetFlameIntensityTimeline)))))))

(fn ConstructionScript)

(fn CalculateRandomTimelineSpeed
  (Components|Timeline|SetPlayRate (Variables|Default|GetFlameIntensityTimeline) (Math|Random|RandomFloatinRange (Variables|Default|GetMinTimelinePlayRate) (Variables|Default|GetMinTimelinePlayRate))))