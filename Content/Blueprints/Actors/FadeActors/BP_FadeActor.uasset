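; Actor whose mesh fades out and back in on request through a timeline scaled to FadeTime.
; Construction caches the original materials and builds dynamic instances from FadeMaterialInstances.
; FadeOut swaps these in and drives their "Fade" parameter, while Fadein reverses the timeline.
; On finish, a custom trace channel and optionally Visibility switch to Ignore or Block by direction, and fading in restores the original materials.
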(event EventBeginPlay
  (Components|Timeline|SetPlayRate (Variables|Default|GetFadeTimeline) (/ 1.0 (Variables|AA|Fade|GetFadeTime))))

(event EventFadein
  (bind (_direction _fade) (Timeline|FadeTimeline Reverse)
    (:Update
      (for _array_element (Variables|AA|Fade|GetDynamicMaterialInstances)
        (Rendering|Material|SetScalarParameterValue _array_element "Fade" _fade :!class /Script/Engine.MaterialInstanceDynamic)))
    (:Finished
      (CallFunction|OnFadeFinished _direction))))

(event EventFadeOut
  (CallFunction|SetMaterialstoDynamicInstances)
  (bind (_direction _fade) (Timeline|FadeTimeline Play)
    (:Update
      (for _array_element (Variables|AA|Fade|GetDynamicMaterialInstances)
        (Rendering|Material|SetScalarParameterValue _array_element "Fade" _fade :!class /Script/Engine.MaterialInstanceDynamic)))
    (:Finished
      (CallFunction|OnFadeFinished _direction))))

(fn ConstructionScript
  (Utilities|Array|Clear (Variables|AA|Fade|GetDynamicMaterialInstances))
  (Variables|AA|Fade|SetOriginalMaterials (Rendering|Material|GetMaterials (Variables|Default|GetMesh)))
  (for _array_element (Variables|AA|Fade|GetFadeMaterialInstances)
    (bind _returnvalue (Rendering|Material|CreateDynamicMaterialInstance _array_element "None" "None" :!class /Script/Engine.KismetMaterialLibrary))
    (Utilities|Array|AddUnique (Variables|AA|Fade|GetDynamicMaterialInstances) _returnvalue)))

(fn SetMaterialstoDynamicInstances
  (for (_array_element _array_index) (Variables|AA|Fade|GetDynamicMaterialInstances)
    (Rendering|Material|SetMaterial (Variables|Default|GetMesh) _array_index _array_element)))

(fn ResetMaterials
  (for (_array_element _array_index) (Variables|AA|Fade|GetOriginalMaterials)
    (Rendering|Material|SetMaterial (Variables|Default|GetMesh) _array_index _array_element)))

(fn OnFadeFinished
  (params (TimelineDirection :type ETimelineDirection%20Enum :default "Forward"))
  (bind _returnvalue (Utilities|Select :Index TimelineDirection :Forward "ECR_Ignore" :Backward "ECR_Block"))
  (Utilities|FlowControl|Sequence
    (:then_0
      (CallFunction|UpdateResponsetoChannel "ECC_GameTraceChannel2" _returnvalue)
      (if (Variables|AA|Fade|GetbModifyVisibilityChannelOnFadeFinished)
        (CallFunction|UpdateResponsetoChannel "ECC_Visibility" _returnvalue)))
    (:then_1
      (switch Utilities|FlowControl|Switch|SwitchonETimelineDirection TimelineDirection
        (:Backward
          (CallFunction|ResetMaterials))))))

(fn UpdateResponsetoChannel
  (params (Channel :type ECollisionChannel%20Enum :default "ECC_WorldStatic") (NewResponse :type ECollisionResponse%20Enum :default "ECR_Ignore"))
  (Collision|SetCollisionResponsetoChannel (Variables|Default|GetMesh) Channel NewResponse))